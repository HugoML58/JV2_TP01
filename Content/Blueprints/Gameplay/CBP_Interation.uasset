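; CBP_Interation is an interaction Blueprint that lets the player use BP_Interactable actors they are aimed at.
; FindInteractable line-traces on Visibility from a supplied origin and direction up to InteractRange, with one-frame debug drawing.
; It stores a hit interactable as SelectedInteractable and shows its interact message, otherwise clearing the selection.
; Starting the IA_Interact input action calls Interact on the selection if it is valid.
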(event `EnhancedInput|/Game/FirstPerson/Input/Actions/IA_Interact`
  (params (ActionValue :type Boolean) (ElapsedSeconds :type "Float (double-precision)") (TriggeredSeconds :type "Float (double-precision)") (InputAction :type "InputAction Object Reference" :default "/Game/FirstPerson/Input/Actions/IA_Interact.IA_Interact"))
  (bind _selectedinteractable (`self.selectedInteractable`))
  (:`Started`
    (`/Engine/EditorBlueprintResources/StandardMacros.IsValid` _selectedinteractable
      (:`Is Valid`
        (`/Game/Blueprints/BP_Interactable.Interact` _selectedinteractable)))))

(fn `FindInteractable`
  (params (Origin :type "Vector Structure") (Direction :type "Vector Structure"))
  (bind (_outhit _returnvalue) (`KismetSystemLibrary.LineTraceSingle` :`Start` Origin :`End` (+ Origin (* Direction (`self.InteractRange`))) :`TraceChannel` "TraceTypeQuery1" :`DrawDebugType` "ForOneFrame"))
  (if _returnvalue
    (bind _asbp_interactable (cast `/Game/Blueprints/BP_Interactable` (`.HitActor` (`GameplayStatics.BreakHitResult` _outhit)))
      (:`then`
        (bind _output_get (set `self.selectedInteractable` _asbp_interactable))
        (`/Game/Blueprints/BP_Interactable.ShowInteractMessage` _output_get))
      (:`CastFailed`
        (set `self.selectedInteractable` null :!label _label)))
    (else
      (goto _label))))