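; Base item pickup Blueprint that interacting actors with an inventory component can collect.
; On BeginPlay it passes the item name from its item data component to the interactable component for display.
; On interaction it tries to add the item data to the sender's inventory, keeping any positive returned amount as its quantity and otherwise calling CollectItem.
; GetMesh exposes the item's static mesh.
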(event `self.ReceiveBeginPlay`
  (`/Game/Blueprints/Gameplay/Interaction/AC_Interactable.SetDisplayName` (`self.AC_Interactable`) (`/Game/Blueprints/Gameplay/Items/AC_ItemData.GetItemName` (`self.CBP_ItemData`))))

(event `self.AC_Interactable.OnInteract`
  (params (sender :type "Actor Object Reference"))
  (bind _returnvalue (`self.GetComponentByClass` sender "/Game/Blueprints/Gameplay/Inventory/AC_Inventory.AC_Inventory_C"))
  (bind _cbp_itemdata (`self.CBP_ItemData`))
  (`/Engine/EditorBlueprintResources/StandardMacros.IsValid` _returnvalue
    (:`Is Valid`
      (bind _remainingamount (`/Game/Blueprints/Gameplay/Inventory/AC_Inventory.TryAddToInventory` _returnvalue (`self.CBP_ItemData`)))
      (if (> _remainingamount 0)
        (set `/Game/Blueprints/Gameplay/Items/AC_ItemData.quantity` _remainingamount _cbp_itemdata)
        (else
          (`/Game/Blueprints/Gameplay/Items/AC_ItemData.CollectItem` _cbp_itemdata))))))

(fn `GetMesh`
  (returns (mesh :type "StaticMesh Object Reference"))
  (return (`StaticMeshComponent.StaticMesh` (`self.SM_Item_Mesh`))))

(fn `UserConstructionScript`
  (`parent.UserConstructionScript`))