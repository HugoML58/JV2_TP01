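; Item data component that links its owning actor to a row in an item data table.
; GetItem looks up the row named by the ItemData handle and returns it on a successful find, and GetItemName returns that row's Name field.
; CollectItem destroys the owning actor.
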(fn `CollectItem`
  (`Actor.K2_DestroyActor` (`self.GetOwner`)))

(fn `GetItem`
  (returns (item :type "/Game/Blueprints/Structures/Item/Struct_Item_Data Structure"))
  (bind (_datatable _rowname) (break `DataTableRowHandle` (`self.ItemData`)))
  (bind _returnvalue (`|GetDataTableRow` _datatable _rowname)
    (:`then`
      (return _returnvalue))))

(fn `GetItemName`
  (returns (name :type Text))
  (return (`.Name_18_FF8B207545347B56BBE85A88F772B086` (break `/Game/Blueprints/Structures/Item/Struct_Item_Data` (`self.GetItem`)))))