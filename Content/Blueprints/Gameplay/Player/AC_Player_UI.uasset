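; Player UI actor component that owns the inventory widget and toggles it open and closed.
; On BeginPlay it creates and builds WBP_Player_Inventory, then forwards the Select and Options input actions to it for grabbing items and showing item options.
; Opening displays the widget, switches the enabled input set and focuses it in Game and UI mode.
; Closing restores game-only input only if the widget confirms it closed.
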(event `self.ReceiveBeginPlay`
  (`self.CreateInventory`))

(event `EnhancedInput|/Game/Others/Input/Actions/Inventory/IA_Select`
  (params (ActionValue :type Boolean) (ElapsedSeconds :type "Float (double-precision)") (TriggeredSeconds :type "Float (double-precision)") (InputAction :type "InputAction Object Reference" :default "/Game/Others/Input/Actions/Inventory/IA_Select.IA_Select"))
  (:`Started`
    (`/Game/UI/Inventory/Inventories/WBP_Player_Inventory.GrabItem` (`self.InventoryUIReference`))))

(event `EnhancedInput|/Game/Others/Input/Actions/Inventory/IA_Options`
  (params (ActionValue :type Boolean) (ElapsedSeconds :type "Float (double-precision)") (TriggeredSeconds :type "Float (double-precision)") (InputAction :type "InputAction Object Reference" :default "/Game/Others/Input/Actions/Inventory/IA_Options.IA_Options"))
  (:`Started`
    (`/Game/UI/Inventory/Inventories/WBP_Player_Inventory.ShowItemOptions` (`self.InventoryUIReference`))))

(fn `CloseInventory`
  (bind _result (`/Game/UI/Inventory/Inventories/WBP_Player_Inventory.CloseInventory` (`self.InventoryUIReference`)))
  (if _result
    (set `self.isInventoryOpen` false)
    (`/Game/Blueprints/Libraries/BPL_InputUtility.EnableInputs` "NewEnumerator0")
    (`WidgetBlueprintLibrary.SetInputMode_GameOnly` (`GameplayStatics.GetPlayerController` 0))))

(fn `CreateInventory`
  (bind _returnvalue (`|CreateWidget` "/Game/UI/Inventory/Inventories/WBP_Player_Inventory.WBP_Player_Inventory_C"))
  (bind _output_get (set `self.InventoryUIReference` _returnvalue))
  (`/Game/UI/Inventory/Inventories/WBP_Player_Inventory.BuildInventory` _output_get))

(fn `ManageInventory`
  (if (`self.isInventoryOpen`)
    (`self.CloseInventory`)
    (else
      (`self.OpenInventory`))))

(fn `OpenInventory`
  (bind _inventoryuireference (`self.InventoryUIReference`))
  (set `self.isInventoryOpen` true)
  (`/Game/Blueprints/Libraries/BPL_InputUtility.EnableInputs` "NewEnumerator1")
  (`WidgetBlueprintLibrary.SetInputMode_GameAndUIEx` (`GameplayStatics.GetPlayerController` 0) _inventoryuireference "DoNotLock" false)
  (`/Game/UI/Inventory/Inventories/WBP_Player_Inventory.DisplayInventory` _inventoryuireference)
  (`UserWidget.AddToViewport` _inventoryuireference 0))