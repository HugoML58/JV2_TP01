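; Player interaction component that detects and triggers interactable actors, and also creates the HUD widget on BeginPlay.
; FindInteractable line-traces on Visibility from a supplied origin and direction, selecting a hit actor's AC_Interactable only when none is selected.
; Found and reset dispatchers announce selection changes, clearing on a miss or non-interactable hit.
; The IA_Interact input calls the selected component's OnInteract with the owner, then resets the selection.
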(event `self.ReceiveBeginPlay`
  (bind _returnvalue (`|CreateWidget` "/Game/UI/WBP_HUD.WBP_HUD_C"))
  (bind _output_get (set `self.HUD` _returnvalue))
  (`UserWidget.AddToViewport` _output_get 0)
  (`self.ResetInteractable`))

(event `EnhancedInput|/Game/FirstPerson/Input/Actions/IA_Interact`
  (params (ActionValue :type Boolean) (ElapsedSeconds :type "Float (double-precision)") (TriggeredSeconds :type "Float (double-precision)") (InputAction :type "InputAction Object Reference" :default "/Game/FirstPerson/Input/Actions/IA_Interact.IA_Interact"))
  (bind _selectedinteractable (`self.selectedInteractable`))
  (:`Started`
    (`/Engine/EditorBlueprintResources/StandardMacros.IsValid` _selectedinteractable
      (:`Is Valid`
        (`/Game/Blueprints/Gameplay/Interaction/AC_Interactable.OnInteract` _selectedinteractable (`self.GetOwner`))
        (`self.ResetInteractable`)))))

(fn `FindInteractable`
  (params (Origin :type "Vector Structure") (Direction :type "Vector Structure"))
  (bind (_outhit _returnvalue) (`KismetSystemLibrary.LineTraceSingle` :`Start` Origin :`End` (+ Origin (* Direction (`self.InteractRange`))) :`TraceChannel` "TraceTypeQuery1" :`DrawDebugType` "ForOneFrame"))
  (if _returnvalue
    (bind _returnvalue_2 (`Actor.GetComponentByClass` (`.HitActor` (`GameplayStatics.BreakHitResult` _outhit)) "/Game/Blueprints/Gameplay/Interaction/AC_Interactable.AC_Interactable_C"))
    (`/Engine/EditorBlueprintResources/StandardMacros.IsValid` _returnvalue_2
      (:`Is Valid`
        (`/Engine/EditorBlueprintResources/StandardMacros.IsValid` (`self.selectedInteractable`)
          (:`Is Not Valid`
            (set `self.selectedInteractable` _returnvalue_2)
            (`self.OnInteractableFound` _returnvalue_2))))
      (:`Is Not Valid`
        (`/Engine/EditorBlueprintResources/StandardMacros.IsValid` (`self.selectedInteractable`) :!label _label
          (:`Is Valid`
            (`self.ResetInteractable`)))))
    (else
      (goto _label))))

(fn `ResetInteractable`
  (set `self.selectedInteractable` null)
  (`self.OnInteractableReseted`))