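; Player inventory component that toggles the inventory screen with the IA_Inventory input action.
; On BeginPlay it creates a WBP_Inventory widget once and maps it to InventorySize.
; Opening fills the cached widget from the Inventory data and adds it to the viewport, while closing removes it.
; Both transitions switch the input mode through EnableInputs and track the IsInventoryOpen flag.
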(event `self.ReceiveBeginPlay`
  (`self.CreateInventory`)
  (`parent.ReceiveBeginPlay`))

(event `EnhancedInput|/Game/FirstPerson/Input/Actions/Inventory/IA_Inventory`
  (params (ActionValue :type Boolean) (ElapsedSeconds :type "Float (double-precision)") (TriggeredSeconds :type "Float (double-precision)") (InputAction :type "InputAction Object Reference" :default "/Game/FirstPerson/Input/Actions/Inventory/IA_Inventory.IA_Inventory"))
  (:`Started`
    (if (`self.isInventoryOpen`)
      (`self.CloseInventory`)
      (else
        (`self.OpenInventory`)))))

(fn `CloseInventory`
  (set `self.isInventoryOpen` false)
  (`/Game/Blueprints/Libraries/BPL_InputUtility.EnableInputs` "NewEnumerator0")
  (`Widget.RemoveFromParent` (`self.InventoryUIReference`)))

(fn `CreateInventory`
  (bind _returnvalue (`|CreateWidget` "/Game/UI/Inventory/WBP_Inventory.WBP_Inventory_C"))
  (bind _output_get (set `self.InventoryUIReference` _returnvalue))
  (`/Game/UI/Inventory/WBP_Inventory.Map Inventory` _output_get (`self.inventorySize`)))

(fn `OpenInventory`
  (bind _inventoryuireference (`self.InventoryUIReference`))
  (set `self.isInventoryOpen` true)
  (`/Game/Blueprints/Libraries/BPL_InputUtility.EnableInputs` "NewEnumerator1")
  (`/Game/UI/Inventory/WBP_Inventory.FillInventory` _inventoryuireference (`self.inventory`))
  (`UserWidget.AddToViewport` _inventoryuireference 0))