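; Blueprint function library that switches the local player's input mode between Gameplay and Inventory.
; EnableInputs swaps Enhanced Input mapping contexts on player 0: Gameplay uses the default and weapons contexts, Inventory uses only the inventory context.
; It also shows the mouse cursor for Inventory and hides it for Gameplay, doing nothing if the input subsystem is invalid.
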(fn `EnableInputs`
  (params (Type :type "/Game/Blueprints/Enums/Enum_InputType Enum" :default "NewEnumerator0"))
  (bind _returnvalue (`GameplayStatics.GetPlayerController` null))
  (bind _returnvalue_2 (pcsubsystem `EnhancedInputLocalPlayerSubsystem` (`GameplayStatics.GetPlayerController` null)))
  (`/Engine/EditorBlueprintResources/StandardMacros.IsValid` _returnvalue_2
    (:`Is Valid`
      (switch `/Game/Blueprints/Enums/Enum_InputType` Type
        (:`NewEnumerator0`
          (`EnhancedInputSubsystemInterface.RemoveMappingContext` _returnvalue_2 "/Game/FirstPerson/Input/IMC_Inventory.IMC_Inventory" (struct))
          (`EnhancedInputSubsystemInterface.AddMappingContext` _returnvalue_2 "/Game/FirstPerson/Input/IMC_Default.IMC_Default" 0 (struct))
          (`EnhancedInputSubsystemInterface.AddMappingContext` _returnvalue_2 "/Game/FirstPerson/Input/IMC_Weapons.IMC_Weapons" 0 (struct))
          (set `PlayerController.bShowMouseCursor` false _returnvalue))
        (:`NewEnumerator1`
          (`EnhancedInputSubsystemInterface.RemoveMappingContext` _returnvalue_2 "/Game/FirstPerson/Input/IMC_Default.IMC_Default" (struct))
          (`EnhancedInputSubsystemInterface.RemoveMappingContext` _returnvalue_2 "/Game/FirstPerson/Input/IMC_Weapons.IMC_Weapons" (struct))
          (`EnhancedInputSubsystemInterface.AddMappingContext` _returnvalue_2 "/Game/FirstPerson/Input/IMC_Inventory.IMC_Inventory" 0 (struct))
          (set `PlayerController.bShowMouseCursor` true _returnvalue))))))